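; Weapon Blueprint that handles automatic firing, magazine ammo and reserve ammo.
; While the 開槍 input is held, a Delay loop spawns BP_子彈 at the mesh's muzzle socket, passes it the weapon damage, plays a particle effect and decrements the magazine.
; Custom event 換彈夾 refills the magazine from the reserve, limited by what remains.
; Custom event 補充子彈 adds one magazine's worth to the reserve, clamped to its cap.
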(event Custom|換彈夾
  ;[0.06373 0.2175 1] 計算要補充幾顆子彈
  (Variables|Default|Set要補充的子彈數量 (- (Variables|Default|Get彈夾尺寸) (Variables|Default|Get目前子彈數量))) ; 計算要補充的子彈數量
  ;[0 0.1346 1] 判斷總數是否大於等於要補充的數量
  (if (>= (Variables|Default|Get子彈總數) (Variables|Default|Get要補充的子彈數量))
    _
    (else
      ;[1 1 1] 總數<要補充的數量
      (Variables|Default|Set要補充的子彈數量 (Variables|Default|Get子彈總數))))
  ;[0 0.1707 1] 目前子彈與總數更新
  (Variables|Default|Set目前子彈數量 (+ (Variables|Default|Get目前子彈數量) (Variables|Default|Get要補充的子彈數量))) ; 補充子但數量
  (Variables|Default|Set子彈總數 (- (Variables|Default|Get子彈總數) (Variables|Default|Get要補充的子彈數量))) ; 扣除子彈總數
)

(event Custom|補充子彈
  ;[1 1 1] 補充子彈
  (bind _output_get (Variables|Default|Set子彈總數 (+ (Variables|Default|Get子彈總數) (Variables|Default|Get彈夾尺寸))))
  (Variables|Default|Set子彈總數 (Math|Integer|Clamp(Integer) _output_get 0 (Variables|Default|Get子彈上限))))

(event Input|ActionEvents|InputAction開槍
  (params (Key :type Key%20Structure :default "None"))
  (bind _sk_ka74u_y (Variables|Default|GetSK_KA74U_Y))
  (bind _returnvalue (Transformation|GetSocketRotation _sk_ka74u_y "None"))
  ;[1 1 1] 開槍
  (:Pressed
    (Variables|Default|Set開槍中 true)
    (if (and (> (Variables|Default|Get目前子彈數量) 0) (Variables|Default|Get開槍中)) :!label _label ; 當目前子但數量大於0才能開槍
      (bind _returnvalue_2 (Game|SpawnActorfromClass "/Game/bp/BP_子彈.BP_子彈_C" (Transformation|GetSocketTransform (Variables|Default|GetSK_KA74U_Y) "子彈插槽" "RTS_World") "Undefined" 0 0)) ; 生成子彈藍圖
      (Variables|/Game/bp/BP_子彈.BP_子彈_C|Set目前武器傷害 _returnvalue_2 (Variables|Default|Get武器傷害))
      (Effects|SpawnEmitteratLocation "/Game/InfinityBladeEffects/Effects/FX_Mobile/Fire/combat/P_FireBall_Powerup.P_FireBall_Powerup" (Transformation|GetSocketLocation _sk_ka74u_y "子彈插槽") (Math|Rotator|MakeRotator (+ (.roll _returnvalue) 9e+01) (.pitch _returnvalue) (+ (.yaw _returnvalue) 9e+01)) "0.100000,0.100000,0.100000")
      (Variables|Default|Set目前子彈數量 (- (Variables|Default|Get目前子彈數量) 1))
      (Utilities|FlowControl|Delay (Variables|Default|Get開槍間隔))
      (goto _label)))
  (:Released
    (Variables|Default|Set開槍中 false)))

(fn ConstructionScript)